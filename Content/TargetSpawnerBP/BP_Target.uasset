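; BP_Target is a shootable target sphere with three ring colours that plays a dissolve effect and destroys itself when hit.
; DestroyTarget passes the impact position and normal to the sphere's material, disables collision and sets a flag.
; Tick then plays a timeline that grows a sphere mask, fades opacity, scales up the actor and blends the rings to a destroy colour before destroying it.
; Older timeline and eased parameter-tick helpers remain unwired.
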(event EventBeginPlay
  (Rendering|Material|SetVectorParameterValueonMaterials (Variables|Default|Gettarget_sphere) "RingColor0" (Variables|Default|GetRingColor0))
  (Rendering|Material|SetVectorParameterValueonMaterials (Variables|Default|Gettarget_sphere) "RingColor1" (Variables|Default|GetRingColor1))
  (Rendering|Material|SetVectorParameterValueonMaterials (Variables|Default|Gettarget_sphere) "RingColor2" (Variables|Default|GetRingColor2)))

(event Collision|EventActorBeginOverlap
  (params (OtherActor :type Actor%20Object%20Reference)))

(event EventTick
  (params (DeltaSeconds :type Float%20%28single-precision%29))
  (if (Variables|Default|GetBeginDestroy)
    (bind _lerpalpha (Timeline|SphereMaskTimeline Play)
      (:Update
        (Rendering|Material|SetScalarParameterValueonMaterials (Variables|Default|Gettarget_sphere) "SphereMaskRadius" (Math|Float|Lerp 0.0 5e+02 _lerpalpha))
        (Rendering|Material|SetScalarParameterValueonMaterials (Variables|Default|Gettarget_sphere) "OpacityOverride" (Math|Float|Lerp 1.0 0.0 _lerpalpha))
        (Transformation|SetActorScale3D (Math|Conversions|ToVector(Float) (Math|Float|Lerp 1.0 1.5 _lerpalpha)))
        (Rendering|Material|SetVectorParameterValueonMaterials (Variables|Default|Gettarget_sphere) "RingColor0" (Math|Vector|Lerp(Vector) (Variables|Default|GetRingColor0) (Variables|Default|GetRingColorDestroy) _lerpalpha))
        (Rendering|Material|SetVectorParameterValueonMaterials (Variables|Default|Gettarget_sphere) "RingColor1" (Math|Vector|Lerp(Vector) (Variables|Default|GetRingColor1) (Variables|Default|GetRingColorDestroy) _lerpalpha))
        (Rendering|Material|SetVectorParameterValueonMaterials (Variables|Default|Gettarget_sphere) "RingColor2" (Math|Vector|Lerp(Vector) (Variables|Default|GetRingColor2) (Variables|Default|GetRingColorDestroy) _lerpalpha)))
      (:Finished
        (Actor|DestroyActor)))))

(fn ConstructionScript)

(fn DestroyTarget
  (params (ImpactNormal :type Vector) (ImpactPosition :type Vector))
  (bind _target_sphere (Variables|Default|Gettarget_sphere))
  (Rendering|Material|SetVectorParameterValueonMaterials _target_sphere "ImpactPosition" ImpactPosition)
  (Rendering|Material|SetVectorParameterValueonMaterials _target_sphere "ImpactNormal" ImpactNormal)
  (Collision|SetCollisionEnabled _target_sphere "NoCollision")
  (Variables|Default|SetBeginDestroy true))

(fn TickMaterialParameter(vector)
  (params (ParameterName :type Name) (Timer :type Float%20%28single-precision%29%20%28by%20ref%29) (Time :type Float%20%28single-precision%29) (From :type Vector%20%28by%20ref%29) (To :type Vector) (DeltaTime :type Float%20%28single-precision%29))
  (if (<= Timer Time)
    (|SetBy-RefVar Timer (+ Timer DeltaTime))
    (Rendering|Material|SetVectorParameterValueonMaterials (Variables|Default|Gettarget_sphere) ParameterName (Math|Vector|Lerp(Vector) From To (CallFunction|EaseOutModifier (/ Timer Time))))))

(fn TickMaterialParameter
  (params (ParameterName :type Name) (Timer :type Float%20%28single-precision%29%20%28by%20ref%29) (Time :type Float%20%28single-precision%29%20%28by%20ref%29) (From :type Float%20%28single-precision%29%20%28by%20ref%29) (To :type Float%20%28single-precision%29%20%28by%20ref%29) (DeltaTime :type Float%20%28single-precision%29%20%28by%20ref%29))
  (if (<= Timer Time)
    (|SetBy-RefVar Timer (+ Timer DeltaTime))
    (Rendering|Material|SetScalarParameterValueonMaterials (Variables|Default|Gettarget_sphere) ParameterName (Math|Float|Lerp From To (CallFunction|EaseOutModifier (/ Timer Time))))))

(fn EaseOutModifier
  (params (Alpha :type Float%20%28single-precision%29))
  (return (* Alpha (- 2.0 Alpha))))

(fn SampleTickFunction
  (params (DeltaTime :type Float%20%28single-precision%29))
  (Development|PrintString (Utilities|String|ToString(Float) DeltaTime)))