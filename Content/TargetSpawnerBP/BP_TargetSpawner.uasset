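; BP_TargetSpawner is an actor that periodically spawns BP_Target actors at random points around itself.
; Tick accumulates a timer and, on reaching SpawnTime, resets it and spawns at the sprite component's location plus a random offset.
; RandomPointInFOV builds that offset by rotating world forward, scaled within min/max radius, by random yaw and pitch inside the configured angles, ignoring the spawner's own rotation.
; The RandomSign helper is unused.
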(event EventBeginPlay)

(event Collision|EventActorBeginOverlap
  (params (OtherActor :type Actor%20Object%20Reference)))

(event EventTick
  (params (DeltaSeconds :type Float%20%28single-precision%29))
  ;[1 1 1] Spawn Timer Tick
  (Variables|Default|SetspawnTimer (+ DeltaSeconds (Variables|Default|GetspawnTimer)))
  (if (>= (Variables|Default|GetspawnTimer) (Variables|Default|GetSpawnTime))
    (Variables|Default|SetspawnTimer 0.0)
    (bind _out (CallFunction|RandomPointinFOV))
    (Game|SpawnActorfromClass "/Game/TargetSpawnerBP/BP_Target.BP_Target_C" (Math|Conversions|ToTransform(Vector) (+ _out (Transformation|GetWorldLocation (Variables|Default|GetSpriteComponent)))) "Undefined" 0 0)))

(fn ConstructionScript)

(fn RandomPointinFOV
  (bind _spawnanglehorizontal (Variables|Default|GetSpawnAngleHorizontal))
  (bind _spawnanglevertical (Variables|Default|GetSpawnAngleVertical))
  (return (Math|Vector|RotateVector (* (Class|KismetMathLibrary|VectorForward) (Math|Random|RandomFloatinRange (Variables|Default|GetSpawnRadiusMin) (Variables|Default|GetSpawnRadiusMax))) (Math|Rotator|MakeRotator 0.0 (Math|Random|RandomFloatinRange (* _spawnanglevertical -0.5) (* _spawnanglevertical 0.5)) (Math|Random|RandomFloatinRange (* _spawnanglehorizontal -0.5) (* _spawnanglehorizontal 0.5))))))

(fn RandomSign
  (if (Math|Random|RandomBool)
    (return -1.0)
    (else
      (return 1.0))))